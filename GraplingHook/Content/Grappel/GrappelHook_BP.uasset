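; GrappelHook_BP is a grappling hook projectile that flies in a straight line toward a Target actor.
; On BeginPlay it records start and end locations and launches its ProjectileMovement along that direction at Speed.
; Tick compares squared distances from the start and, once the Target's distance is reached, snaps to the stored end point and zeroes velocity.
; DistanceToTarget returns the remaining distance to that stored end point.
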(event EventBeginPlay
  (Variables|Privat|SetStartinglocation (Transformation|GetActorLocation))
  (Variables|Privat|SetEndinglocation (Transformation|GetActorLocation (Variables|Default|GetTarget)))
  (Variables|Privat|SetDirection (Math|Vector|Normalize (- (Variables|Privat|GetEndinglocation) (Variables|Privat|GetStartinglocation))))
  (Variables|/Script/Engine.MovementComponent|SetVelocity (Variables|Default|GetProjectileMovement) (* (Variables|Privat|GetDirection) (Variables|Default|GetSpeed))))

(event EventTick
  (params (DeltaSeconds :type Float%20%28single-precision%29))
  (if (>= (Class|KismetMathLibrary|VectorDistanceSquared (Transformation|GetActorLocation) (Variables|Privat|GetStartinglocation)) (Class|KismetMathLibrary|VectorDistanceSquared (Transformation|GetActorLocation (Variables|Default|GetTarget)) (Variables|Privat|GetStartinglocation)))
    (Transformation|SetActorLocation (+ (Variables|Privat|GetStartinglocation) (* (Variables|Privat|GetDirection) (Math|Vector|Distance(Vector) (Variables|Privat|GetStartinglocation) (Variables|Privat|GetEndinglocation)))) false false)
    (Variables|/Script/Engine.MovementComponent|SetVelocity (Variables|Default|GetProjectileMovement) "0, 0, 0")))

(fn ConstructionScript)

(fn DistancetoTarget
  (return (Math|Vector|Distance(Vector) (Variables|Privat|GetEndinglocation) (Transformation|GetActorLocation))))