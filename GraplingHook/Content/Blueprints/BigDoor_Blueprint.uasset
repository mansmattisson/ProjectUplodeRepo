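; BigDoor is a door Blueprint that the player opens and closes while overlapping its Box trigger.
; Overlap enables input for player controller 0 and end overlap disables it.
; E and the gamepad left face button toggle a shared DoorClosed flag, playing or reversing a timeline that sets the Door's relative location.
; Each input drives its own separate timeline rather than sharing one.
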(event OnComponentBeginOverlap(Box)
  (params (OverlappedComponent :type Primitive%20Component%20Object%20Reference) (OtherActor :type Actor%20Object%20Reference) (OtherComp :type Primitive%20Component%20Object%20Reference) (OtherBodyIndex :type Integer) (bFromSweep :type Boolean) (SweepResult :type Hit%20Result%20Structure%20%28by%20ref%29))
  (Input|EnableInput (Game|GetPlayerController 0)))

(event OnComponentEndOverlap(Box)
  (params (OverlappedComponent :type Primitive%20Component%20Object%20Reference) (OtherActor :type Actor%20Object%20Reference) (OtherComp :type Primitive%20Component%20Object%20Reference) (OtherBodyIndex :type Integer))
  (Input|DisableInput (Game|GetPlayerController 0)))

(event Input|KeyboardEvents|E
  (params (Key :type Key%20Structure :default "None"))
  (:Pressed
    (if (Variables|Default|GetDoor_Closed)
      (Variables|Default|SetDoor_Closed false)
      (bind _open_close_door (Timeline|Open/Close%20door Play)
        (:Update
          (Transformation|SetRelativeLocation (Variables|Default|GetDoor) _open_close_door false false)))
      (else
        (Variables|Default|SetDoor_Closed true)
        (Timeline|Open/Close%20door Reverse)))))

(event Input|GamepadEvents|GamepadFaceButtonLeft
  (params (Key :type Key%20Structure :default "None"))
  (:Pressed
    (if (Variables|Default|GetDoor_Closed)
      (Variables|Default|SetDoor_Closed false)
      (bind _open_close_door (Timeline|Timeline_0 Play)
        (:Update
          (Transformation|SetRelativeLocation (Variables|Default|GetDoor) _open_close_door false false)))
      (else
        (Variables|Default|SetDoor_Closed true)
        (Timeline|Timeline_0 Reverse)))))

(fn ConstructionScript)